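; Actor component that simulates burning on its owner, with random self-ignition and spread to other burning components.
; On a throttled tick, an unlit component rolls to combust, while a lit one rolls to raise the clamped fire counter of each spreadable target.
; Burning also runs a randomized damage countdown, but its expiry only resets it; the TakeDamage function is never called here.
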(event EventBeginPlay
  (Class|ActorComponent|SetComponentTickInterval (Variables|Default|GetTickSpeed))
  (CallFunction|ResetDamageTick))

(event EventTick
  (params (DeltaSeconds :type Float%20%28single-precision%29))
  (if (> (Variables|Default|GetFireCounter) 0)
    (CallFunction|DamageTick)
    (CallFunction|TrySpreadFire)
    (else
      (CallFunction|TryCombust))))

(fn TakeDamage
  (Game|Damage|ApplyDamage (Components|GetOwner) 1.0 0 0))

(fn TryCombust
  (if (> (Variables|Default|GetCombustChance) (Math|Random|RandomFloatinRange 0.0 1.0))
    (CallFunction|ChangeFireCounter 1)))

(fn TrySpreadFire
  (for _array_element (Variables|Default|GetSpreadableTargets)
    (if (> (Variables|Default|GetSpreadChance) (Math|Random|RandomFloatinRange 0.0 1.0))
      (CallFunction|ChangeFireCounter _array_element 1))))

(fn ChangeFireCounter
  (params (Change :type Integer))
  (Variables|Default|SetFireCounter (Math|Integer|Clamp(Integer) (+ Change (Variables|Default|GetFireCounter)) 0 (Variables|Default|GetMaxFireCounter))))

(fn DamageTick
  (bind _result (Math|Integer|DecrementInt (Variables|Default|GetTicksUntilDamage))
    (:%20%20
      (if (<= _result 0)
        (CallFunction|ResetDamageTick)))))

(fn ResetDamageTick
  (bind _baseticksfordamage (Variables|Default|GetBaseTicksForDamage))
  (bind _randomoffsetrangeticksfordamage (Variables|Default|GetRandomOffsetRangeTicksForDamage))
  (Variables|Default|SetTicksUntilDamage (Math|Random|RandomIntegerinRange (- _baseticksfordamage _randomoffsetrangeticksfordamage) (+ _baseticksfordamage _randomoffsetrangeticksfordamage))))